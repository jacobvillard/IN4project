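; Pickup child Blueprint that overrides OverlapLogic with one of two responses, chosen by the ScaleBehaviour flag.
; When set, it increases Score and Scale by their increment variables, playing a sound only while Scale is at or below a threshold.
; Otherwise, it swaps the Cube to a random mesh from StaticMeshes and plays the same sound.
; Its event graph holds only disabled placeholder nodes.
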(fn `OverlapLogic`
  (bind _scale (`self.Scale`))
  (bind _staticmeshes (`self.StaticMeshes`))
  (if (`self.ScaleBehaviour`)
    (if (<= _scale 30)
      (`GameplayStatics.PlaySound2D` "/Engine/EditorSounds/GamePreview/EndPlayInEditor.EndPlayInEditor" 1.0 1.0 0.0 null null))
    (set `self.Score` (+ (`self.Score`) (`self.ScoreIncrease`)))
    (set `self.Scale` (+ _scale (`self.ScaleIncrease`)))
    (else
      (`StaticMeshComponent.SetStaticMesh` (`self.Cube`) (`|GetArrayItem` _staticmeshes (`KismetMathLibrary.RandomInteger` (`KismetArrayLibrary.Array_Length` _staticmeshes))))
      (`GameplayStatics.PlaySound2D` "/Engine/EditorSounds/GamePreview/EndPlayInEditor.EndPlayInEditor" 1.0 1.0 0.0 null null))))

(fn `UserConstructionScript`
  (`parent.UserConstructionScript`))