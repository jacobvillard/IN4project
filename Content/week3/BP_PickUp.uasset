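; BP_PickUp is a pickup actor whose overlap event only casts to BP_ThirdPersonCharacter, with the pickup sequence left disconnected.
; That unwired sequence hides the actor, disables collision, triggers optional audio and Niagara effects through OverlapLogic, and waits for a delay.
; It then moves to a random point in a box or radius, absolute or relative to its location, and reappears with set scale and optional material.
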(event `self.ReceiveActorBeginOverlap`
  (params (OtherActor :type "Actor Object Reference"))
  (cast `/Game/ThirdPerson/Blueprints/BP_ThirdPersonCharacter` OtherActor))

(fn `OverlapLogic`
  (if (`self.PlaySound`)
    (`ActorComponent.Activate` (`self.Audio`) false))
  (if (`self.PlayVFX`)
    (`ActorComponent.Activate` (`self.Niagara`) false)))

(fn `UserConstructionScript`)