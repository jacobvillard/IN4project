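; BP_PickUp_Constuction is a pickup-named actor whose look is randomized in its construction script, with no active gameplay logic.
; It assigns the Cube a random material from the Materials array and gives the PointLight a random RGB color.
; Light intensity and attenuation radius are random integers drawn between configurable min and max variables.
; Randomization uses unseeded functions, so results reroll whenever the construction script reruns.
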(fn `UserConstructionScript`
  (bind _materials (`self.Materials`))
  (bind _pointlight (`self.PointLight`))
  (`parent.UserConstructionScript`)
  (`PrimitiveComponent.SetMaterial` (`self.Cube`) 0 (`|GetArrayItem` _materials (`KismetMathLibrary.RandomInteger` (`KismetArrayLibrary.Array_Length` _materials))))
  (`LightComponent.SetLightColor` _pointlight (`KismetMathLibrary.MakeColor` (`KismetMathLibrary.RandomFloatInRange` 0.0 1.0) (`KismetMathLibrary.RandomFloatInRange` 0.0 1.0) (`KismetMathLibrary.RandomFloatInRange` 0.0 1.0)) true)
  (`LightComponent.SetIntensity` (`self.PointLight`) (`KismetMathLibrary.Conv_Int64ToDouble` (`KismetMathLibrary.RandomInteger64InRange` (`self.MinIntensity`) (`self.MaxIntensity`))))
  (`LocalLightComponent.SetAttenuationRadius` _pointlight (`KismetMathLibrary.Conv_Int64ToDouble` (`KismetMathLibrary.RandomInteger64InRange` (`self.MinAttRadius`) (`self.MaxAttRadius`)))))